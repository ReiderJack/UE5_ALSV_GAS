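; GA_Jump is a Gameplay Ability that makes the AnimMan character from an ALSV GAS setup jump.
; On activation it caches the owning character, then cancels if the character is falling or otherwise commits, triggering JumpPressed from CommitExecute.
; It waits for input release to end the ability, and ending calls StopJumping so the jump follows how long input is held.
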(event `self.K2_ActivateAbility`
  (bind _asanim_man_character_bp (cast `/Game/ALSV_GAS/Blueprints/Character/AnimMan_CharacterBP` (`self.GetOwningActorFromActorInfo`)))
  (bind _output_get (set `self.As Anim Man Character BP` _asanim_man_character_bp))
  (if (`NavMovementComponent.IsFalling` (`Character.CharacterMovement` _output_get))
    (`self.K2_CancelAbility`)
    (else
      (`self.K2_CommitAbility`)
      (`AbilityTask_WaitInputRelease.WaitInputRelease` false
        (:`OnRelease`
          (`self.K2_EndAbility`))))))

(event `self.K2_CommitExecute`
  (`/Game/ALSV_GAS/Blueprints/Character/Base_CharacterBP.Jump_Pressed` (`self.As Anim Man Character BP`)))

(event `self.K2_OnEndAbility`
  (params (bWasCancelled :type Boolean))
  (`Character.StopJumping` (`self.As Anim Man Character BP`)))