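; Gameplay Ability for sprinting that sets the character's desired gait to Sprinting and restores Running when it ends.
; Activation requires stamina above a small threshold, then commits the ability, which removes the stamina regen effect.
; A looping timer repeatedly commits the cost until input release or empty stamina ends the ability.
; Ending clears the timer, removes the sprint cost effect and reapplies stamina regen.
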(event `self.K2_ActivateAbility`
  (if (`self.HasStamina`)
    (if (> (`.CurrentValue` (break `GameplayAttributeData` (`BaseAttributeSet.Stamina` (`self.BaseAttributeSet`)))) 5.0)
      (`self.K2_CommitAbility`)
      (`AbilityTask_WaitInputRelease.WaitInputRelease` false
        (:`then`
          (bind _returnvalue (`KismetSystemLibrary.K2_SetTimerDelegate` (delegate `SprintCost`) 0.1 true false 0.1))
          (set `self.CostTimer` _returnvalue))
        (:`OnRelease`
          (`self.K2_EndAbility`)))
      (else
        (`self.K2_CancelAbility`)))
    (else
      (`self.K2_CancelAbility`))))

(event `SprintCost`
  (`self.K2_CommitAbilityCost` false)
  (if (not (`self.HasStamina`))
    (`self.K2_EndAbility`)))

(event `self.K2_CommitExecute`
  (`AbilitySystemComponent.RemoveActiveGameplayEffectBySourceEffect` (`AbilitySystemBlueprintLibrary.GetAbilitySystemComponent` (`self.GetCharacterBase`)) "/Game/ALSV_GAS/Blueprints/Abilitites/Effects/GE_Stamina_Regen.GE_Stamina_Regen_C" null -1)
  (`ALSBaseCharacter.SetDesiredGait` (`self.GetCharacterBase`) "Sprinting"))

(event `CheckStamina`
  (if (not (`self.HasStamina`))
    (`self.K2_EndAbility`)))

(event `self.K2_OnEndAbility`
  (params (bWasCancelled :type Boolean))
  (bind _returnvalue (`AbilitySystemBlueprintLibrary.GetAbilitySystemComponent` (`self.GetCharacterBase`)))
  (`ALSBaseCharacter.SetDesiredGait` (`self.GetCharacterBase`) "Running")
  (`AbilitySystemComponent.RemoveActiveGameplayEffectBySourceEffect` _returnvalue "/Game/ALSV_GAS/Blueprints/Abilitites/Effects/GE_Sprint_Cost.GE_Sprint_Cost_C" null -1)
  (`AbilitySystemComponent.BP_ApplyGameplayEffectToSelf` :`self` _returnvalue :`GameplayEffectClass` "/Game/ALSV_GAS/Blueprints/Abilitites/Effects/GE_Stamina_Regen.GE_Stamina_Regen_C" :`Level` 1.0)
  (`KismetSystemLibrary.K2_ClearAndInvalidateTimerHandle` (`self.CostTimer`)))

(fn `HasStamina`
  (returns (HasStamina :type Boolean))
  (`/Engine/EditorBlueprintResources/StandardMacros.IsValid` (`self.BaseAttributeSet`)
    (:`Is Valid`
      _)
    (:`Is Not Valid`
      (bind _returnvalue (`AbilitySystemComponent.GetAttributeSet` (`CharacterBase.AbilitySystemComponent` (`self.GetCharacterBase`)) "/Script/ALSV_GAS.BaseAttributeSet"))
      (bind _asbase_attribute_set (cast `BaseAttributeSet` _returnvalue)
        (:`then`
          (set `self.BaseAttributeSet` _asbase_attribute_set))
        (:`CastFailed`
          (return false)))))
  (return (> (`.CurrentValue` (break `GameplayAttributeData` (`BaseAttributeSet.Stamina` (`self.BaseAttributeSet`)))) 0.0)))