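; GAS dash ability that launches the ALS character forward with a Niagara effect and randomly pitched whoosh sound.
; On successful commit it caches velocity, sets velocity along actor forward, and adds an impulse along camera forward.
; It ends immediately, and OnEndAbility deactivates the effect and restores the cached velocity.
; A cooldown widget is created only without authority; force-based and delayed-reset variants are left unconnected.
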(event `self.K2_ActivateAbility`
  (bind _returnvalue (`Actor.GetComponentByClass` (`self.Anim Man Character BP`) "/Script/Niagara.NiagaraComponent"))
  (bind _asanim_man_character_bp (cast `/Game/ALSV_GAS/Blueprints/Character/AnimMan_CharacterBP` (`self.GetAvatarActorFromActorInfo`)))
  (set `self.Anim Man Character BP` _asanim_man_character_bp)
  (bind _returnvalue_2 (`self.K2_CommitAbility`))
  (if _returnvalue_2
    (set `self.OriginalVelocity` (`MovementComponent.Velocity` (`Character.CharacterMovement` (`self.Anim Man Character BP`))))
    (`|ExecutionSequence`
      (:`then_0`
        (`self.K2_HasAuthority`
          (:`False`
            (bind _returnvalue_3 (`|CreateWidget` "/Game/ALSV_GAS/Blueprints/Widget/UW_CoolDown.UW_CoolDown_C" null 2.0 "/Game/ALSV_GAS/Texture/DashImage.DashImage"))
            (`UserWidget.AddToViewport` _returnvalue_3 0))))
      (:`then_1`
        (`/Engine/EditorBlueprintResources/StandardMacros.IsValid` _returnvalue
          (:`Is Valid`
            (bind _output_get (set `self.NiagaraEffect` _returnvalue))
            (`ActorComponent.Activate` _output_get true))))
      (:`then_2`
        (`GameplayStatics.PlaySoundAtLocation` "/Game/ALSV_GAS/Audio/whoosh-dash.whoosh-dash" (`SceneComponent.K2_GetComponentLocation` (`Character.Mesh` (`self.Anim Man Character BP`))) (struct) 1.0 (`KismetMathLibrary.RandomFloatInRange` 0.4 1.0) 0.0 null null null null))
      (:`then_3`
        (set `MovementComponent.Velocity` (* (`Actor.GetActorForwardVector` (`self.GetAvatarActorFromActorInfo`)) (`self.Strength`)) (`Character.CharacterMovement` (`self.Anim Man Character BP`)))
        (`CharacterMovementComponent.AddImpulse` (`Character.CharacterMovement` (`self.Anim Man Character BP`)) (* (`SceneComponent.GetForwardVector` (`/Game/ALSV_GAS/Blueprints/Character/AnimMan_CharacterBP.Camera` (`self.Anim Man Character BP`))) (`self.Strength`)) false)
        (`self.K2_EndAbility`)))
    (else
      (`self.K2_CancelAbility`))))

(event `self.K2_OnEndAbility`
  (params (bWasCancelled :type Boolean))
  (bind _niagaraeffect (`self.NiagaraEffect`))
  (`|ExecutionSequence`
    (:`then_0`
      (`/Engine/EditorBlueprintResources/StandardMacros.IsValid` _niagaraeffect
        (:`Is Valid`
          (`ActorComponent.Deactivate` _niagaraeffect))))
    (:`then_1`
      (set `MovementComponent.Velocity` (`self.OriginalVelocity`) (`Character.CharacterMovement` (`self.Anim Man Character BP`))))))