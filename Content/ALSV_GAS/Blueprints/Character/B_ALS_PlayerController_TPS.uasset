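; Player controller for the third-person ALS and GAS character, providing a respawn for the controlled pawn.
; Respawn unpossesses and destroys the current pawn through DestroyCurrentPawn, then spawns a new B_CharacterBase at the PlayerStart returned by GetActorOfClass.
; The controller then possesses the new character and enables input.
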(event `Respawn`
  (`self.DestroyCurrentPawn`)
  (bind _returnvalue (`GameplayStatics.GetActorOfClass` "/Script/Engine.PlayerStart"))
  (bind _returnvalue_2 (`|SpawnActorFromClass` "/Game/ALSV_GAS/Blueprints/Character/B_CharacterBase.B_CharacterBase_C" (`self.GetTransform` _returnvalue) "Undefined" "MultiplyWithRoot" self null))
  (`self.Possess` _returnvalue_2)
  (`self.EnableInput` self))

(event `DestroyCurrentPawn`
  (set `self.CurrentPawn` (`self.K2_GetPawn`))
  (`self.UnPossess`)
  (`self.K2_DestroyActor` (`self.CurrentPawn`)))

(fn `UserConstructionScript`
  (`parent.UserConstructionScript`))